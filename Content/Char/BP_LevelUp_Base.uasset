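; BP_LevelUp_Base is a trigger actor that shows the level-up UI while the player character stands inside its box.
; Box overlap events check that the other actor's class is TryNewChar, opening BP_UI_LvlUp on entry and BP_UI_Main on exit.
; Each switch removes all widgets, then creates and adds a fresh widget to the viewport.
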(event OnComponentBeginOverlap(Box)
  (params (OverlappedComponent :type Primitive%20Component%20Object%20Reference) (OtherActor :type Actor%20Object%20Reference) (OtherComp :type Primitive%20Component%20Object%20Reference) (OtherBodyIndex :type Integer) (bFromSweep :type Boolean) (SweepResult :type Hit%20Result%20Structure%20%28by%20ref%29))
  (if (== (Utilities|GetClass OtherActor) "/Game/Animationtry/TryNewChar.TryNewChar_C")
    (CallFunction|LvlUpViewport)))

(event OnComponentEndOverlap(Box)
  (params (OverlappedComponent :type Primitive%20Component%20Object%20Reference) (OtherActor :type Actor%20Object%20Reference) (OtherComp :type Primitive%20Component%20Object%20Reference) (OtherBodyIndex :type Integer))
  (if (== (Utilities|GetClass OtherActor) "/Game/Animationtry/TryNewChar.TryNewChar_C")
    (CallFunction|MainViewPort)))

(event EventBeginPlay)

(event Collision|EventActorBeginOverlap
  (params (OtherActor :type Actor%20Object%20Reference)))

(event EventTick
  (params (DeltaSeconds :type Float%20%28single-precision%29)))

(fn ConstructionScript)

(fn LvlUpViewport
  (Viewport|RemoveAllWidgets)
  (bind _returnvalue (UserInterface|CreateWidget "/Game/UI/BP_UI_LvlUp.BP_UI_LvlUp_C"))
  (UserInterface|Viewport|AddtoViewport _returnvalue 0))

(fn MainViewPort
  (Viewport|RemoveAllWidgets)
  (bind _returnvalue (UserInterface|CreateWidget "/Game/UI/BP_UI_Main.BP_UI_Main_C"))
  (UserInterface|Viewport|AddtoViewport _returnvalue 0))
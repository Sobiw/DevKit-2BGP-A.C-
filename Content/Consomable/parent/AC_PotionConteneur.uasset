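; AC_PotionConteneur is a component on BP_PlayableCharacter that holds and consumes healing and damage potions.
; The Heal and BuffDmg events take the potion at array index 1, destroy its actor and remove it.
; Healing adds Life capped at MaxLife, while damage potions raise AtkUse if no buff is active.
; Tick counts down the buff time, then removes the bonus once, guarded by IsReset.
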(event Custom|Heal
  (CallFunction|UseHealPotion))

(event Custom|BuffDmg
  (CallFunction|UseDmgPotion))

(event EventBeginPlay
  (bind _asbp_playable_character (Utilities|Casting|CastToBP_PlayableCharacter (Components|GetOwner)))
  (Variables|Default|SetOwner _asbp_playable_character)
  (Variables|Default|SetDmg_Potion (Utilities|Array|MakeArray 0))
  (Variables|Default|SetHeal_Potion (Utilities|Array|MakeArray 0)))

(event EventTick
  (params (DeltaSeconds :type Float%20%28single-precision%29))
  (if (>= (Variables|Default|GetBuffTime) 0.0)
    (Variables|Default|SetBuffTime (- (Variables|Default|GetBuffTime) DeltaSeconds))
    (Variables|Default|SetIsBuff true)
    (else
      (CallFunction|EndDmgPotion))))

(fn UseHealPotion
  (bind _heal_potion (Variables|Default|GetHeal_Potion))
  (bind _owner (Variables|Default|GetOwner))
  (bind _output (Utilities|Array|Get(acopy) _heal_potion 1))
  (bind _maxlife (Variables|/Game/BP_PlayableCharacter.BP_PlayableCharacter_C|GetMaxLife _owner))
  (if (>= (Utilities|Array|Length _heal_potion) 1)
    (bind _asheal_consomable (Utilities|Casting|CastToHeal_Consomable _output))
    (bind _output_get (Variables|Default|SethealPower (Variables|/Game/Consomable/Heal_Consomable.Heal_Consomable_C|GetHealPower _asheal_consomable)))
    (Actor|DestroyActor _output)
    (Utilities|Array|RemoveIndex _heal_potion 1)
    (bind _output_get_2 (Variables|/Game/BP_PlayableCharacter.BP_PlayableCharacter_C|SetLife _owner (+ _output_get (Variables|/Game/BP_PlayableCharacter.BP_PlayableCharacter_C|GetLife _owner))))
    (if (> _output_get_2 _maxlife)
      (Variables|/Game/BP_PlayableCharacter.BP_PlayableCharacter_C|SetLife (Variables|Default|GetOwner) _maxlife))))

(fn UseDmgPotion
  (bind _owner (Variables|Default|GetOwner))
  (bind _dmg_potion (Variables|Default|GetDmg_Potion))
  (bind _output (Utilities|Array|Get(acopy) _dmg_potion 1))
  (if (and (>= (Utilities|Array|Length _dmg_potion) 1) (not (Variables|Default|GetIsBuff)))
    (bind _asdmg_consomable (Utilities|Casting|CastToDmg_Consomable _output))
    (Variables|Default|SetBuffTime (Variables|/Game/Consomable/Dmg_Consomable.Dmg_Consomable_C|GetBuffTime _asdmg_consomable))
    (Variables|Default|SetatkBuffPower (Variables|/Game/Consomable/Dmg_Consomable.Dmg_Consomable_C|GetAtkBuff _asdmg_consomable))
    (Actor|DestroyActor _output)
    (Utilities|Array|RemoveIndex _dmg_potion 1)
    (Variables|/Game/BP_PlayableCharacter.BP_PlayableCharacter_C|SetAtk_Use _owner (+ (Variables|/Game/BP_PlayableCharacter.BP_PlayableCharacter_C|GetAtk_Use _owner) (Variables|/Game/Consomable/Dmg_Consomable.Dmg_Consomable_C|GetAtkBuff _asdmg_consomable)))
    (Variables|Default|SetIsBuff true)
    (Variables|Default|SetIsReset false)))

(fn EndDmgPotion
  (bind _owner (Variables|Default|GetOwner))
  (if (not (Variables|Default|GetIsReset))
    (Variables|/Game/BP_PlayableCharacter.BP_PlayableCharacter_C|SetAtk_Use _owner (- (Variables|/Game/BP_PlayableCharacter.BP_PlayableCharacter_C|GetAtk_Use _owner) (Variables|Default|GetatkBuffPower)))
    (Variables|Default|SetIsBuff false)
    (Variables|Default|SetIsReset true)))
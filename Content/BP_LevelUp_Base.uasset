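; BP_LevelUp_Base is a level-up station that opens the level-up menu while the player character stands inside its box trigger.
; On overlap it clears all widgets, shows BP_UI_LvlUp, sets the character's Shopping flag and shows the mouse cursor.
; Leaving the box reverses this, recreating BP_UI_Main and clearing both the flag and cursor.
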(event OnComponentBeginOverlap(Box)
  (params (OverlappedComponent :type Primitive%20Component%20Object%20Reference) (OtherActor :type Actor%20Object%20Reference) (OtherComp :type Primitive%20Component%20Object%20Reference) (OtherBodyIndex :type Integer) (bFromSweep :type Boolean) (SweepResult :type Hit%20Result%20Structure%20%28by%20ref%29))
  (if (== (Utilities|GetClass OtherActor) "/Game/BP_PlayableCharacter.BP_PlayableCharacter_C")
    (CallFunction|LvlUpViewport)
    (bind _returnvalue (Actor|GetActorOfClass "/Game/BP_PlayableCharacter.BP_PlayableCharacter_C"))
    (bind _asbp_playable_character (Utilities|Casting|CastToBP_PlayableCharacter _returnvalue))
    (Variables|/Game/BP_PlayableCharacter.BP_PlayableCharacter_C|SetShopping _asbp_playable_character true)
    (Variables|/Script/Engine.PlayerController|SetbShowMouseCursor (Game|GetPlayerController 0) true)))

(event OnComponentEndOverlap(Box)
  (params (OverlappedComponent :type Primitive%20Component%20Object%20Reference) (OtherActor :type Actor%20Object%20Reference) (OtherComp :type Primitive%20Component%20Object%20Reference) (OtherBodyIndex :type Integer))
  (if (== (Utilities|GetClass OtherActor) "/Game/BP_PlayableCharacter.BP_PlayableCharacter_C")
    (CallFunction|MainViewPort)
    (bind _returnvalue (Actor|GetActorOfClass "/Game/BP_PlayableCharacter.BP_PlayableCharacter_C"))
    (bind _asbp_playable_character (Utilities|Casting|CastToBP_PlayableCharacter _returnvalue))
    (Variables|/Game/BP_PlayableCharacter.BP_PlayableCharacter_C|SetShopping _asbp_playable_character false)
    (Variables|/Script/Engine.PlayerController|SetbShowMouseCursor (Game|GetPlayerController 0) false)))

(event EventBeginPlay)

(event Collision|EventActorBeginOverlap
  (params (OtherActor :type Actor%20Object%20Reference)))

(event EventTick
  (params (DeltaSeconds :type Float%20%28single-precision%29)))

(fn ConstructionScript)

(fn LvlUpViewport
  (Viewport|RemoveAllWidgets)
  (bind _returnvalue (UserInterface|CreateWidget "/Game/UI/BP_UI_LvlUp.BP_UI_LvlUp_C"))
  (UserInterface|Viewport|AddtoViewport _returnvalue 0))

(fn MainViewPort
  (Viewport|RemoveAllWidgets)
  (bind _returnvalue (UserInterface|CreateWidget "/Game/UI/BP_UI_Main.BP_UI_Main_C"))
  (UserInterface|Viewport|AddtoViewport _returnvalue 0))